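; Base resource actor that takes its data and appearance from a row in the DT_Resources data table and can be selected.
; On BeginPlay it looks up its RowName, stores the row as ResourceData, and applies the visual mesh and relative scale to its StaticMesh.
; Select returns a selection UI struct built from the resource's type, icon and quantity, while DeSelect is an empty event.
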(event EventBeginPlay
  (bind _returnvalue (Utilities|GetDataTableRow "/Game/DataTables/DT_Resources.DT_Resources" (Variables|Default|GetRow%20Name))
    (:then
      (bind _output_get (Variables|Default|SetResourceData _returnvalue))
      (Transformation|SetRelativeScale3D (Variables|Default|GetStaticMesh) (Utilities|Struct|BreakS_Resources _output_get))
      (Components|StaticMesh|SetStaticMesh (Variables|Default|GetStaticMesh) (Utilities|ResolveSoftReference (Utilities|Struct|BreakS_Resources (Variables|Default|GetResourceData)))))))

(event Collision|EventActorBeginOverlap
  (params (OtherActor :type Actor%20Object%20Reference)))

(event EventTick
  (params (DeltaSeconds :type Float%20%28single-precision%29)))

(event EventDeSelect)

(fn ConstructionScript)

(fn Select
  (bind _resourcedata (Variables|Default|GetResourceData))
  (bind (_name _icon _quantity _type) (Utilities|Struct|BreakS_Resources _resourcedata))
  (return (Utilities|Struct|MakeS_SelectedUIData "resource" "NewEnumerator1" _type _icon (Utilities|Map|MakeMap "NewEnumerator0" (Math|Conversions|ToFloat(Integer) _quantity))) "NewEnumerator0" 0))