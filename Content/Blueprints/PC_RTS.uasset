(event Custom|AddMappingContext
  (Utilities|FlowControl|Delay 0.2)
  (Input|AddMappingContext (PlayerController|LocalPlayerSubsystems|GetEnhancedInputLocalPlayerSubsystem) "/Game/Inputs/IMC_Pawn.IMC_Pawn" 0 "(bIgnoreAllPressedKeysUntilRelease=True,bForceImmediately=False,bNotifyUserSettings=False)"))

(event Custom|SetWorldCursorlocation
  (params (NewLocation :type Vector))
  (bind _worldcursor (Variables|Default|GetWorldCursor)
    (:then
      (Default|SetCustomNewLocation _worldcursor (Math|Vector|MakeVector (.x NewLocation) (.y NewLocation) (+ (.z NewLocation) 1.0)) 0.01 (Variables|Default|GetTimeToRefresh)))
    (:else)))

(event Custom|SpawnWorldCursor
  (bind _returnvalue (Game|SpawnActorfromClass "/Game/Blueprints/Player/BP_WorldCursor.BP_WorldCursor_C" (Math|Transform|MakeTransform "0, 0, 0" "0, 0, 0" "1.000000,1.000000,1.000000") "Undefined" "MultiplyWithRoot" self (Variables|Default|GetPlayerName) (Variables|Default|GetPlayerColor) 0))
  (Variables|Default|SetWorldCursor _returnvalue))

(event Custom|RefresCrusorLocation
  (if (== self (Game|GetPlayerController 0))
    (CallFunction|SetWorldCursorlocation (.Location (Collision|BreakHitResult (.HitResult (Game|Player|GetHitResultUnderCursorbyChannel "TraceTypeQuery1" false)))))))

(event EventBeginPlay
  (CallFunction|AddMappingContext)
  (Input|SetInputModeGameandUI self 0 "DoNotLock" false false)
  (Variables|Default|SetbShowMouseCursor true)
  (Utilities|Time|SetTimerbyEvent (EventDispatchers|CreateEvent :!event Custom|RefresCrusorLocation) (Variables|Default|GetTimeToRefresh) true))

(event EventTick
  (params (DeltaSeconds :type Float%20%28single-precision%29)))

(event Custom|UIOnSelectableSelected
  (params (UIStruct :type S%20Selected%20UI%20Data%20Structure) (Actions :type Array%20of%20E_Actions%20Enums :default "NewEnumerator0") (Crafteables :type Array%20of%20Names))
  (Default|SomthingSelected (CallFunction|GetHudRef) UIStruct Actions Crafteables))

(event Custom|ConfirmBuidingPreview
  (params (Spawn%20Transform%20Location :type Vector) (IDBuilding :type Name))
  (Default|SpawnBuildforPlayer (CallFunction|GetGSRef) self IDBuilding Spawn%20Transform%20Location))

(event Custom|ConfirmBuilding
  (bind _previewbuilding (Variables|Default|GetPreviewBuilding)
    (:then
      (if (and (Default|CaniBuildHere _previewbuilding) (Default|CanIPayIt _previewbuilding))
        (CallFunction|ConfirmBuidingPreview (CallFunction|GetCursorLocation "TraceTypeQuery4") (Variables|/Game/Blueprints/Buildings/BP_BaseBuilding.BP_BaseBuilding_C|GetIDBuilding (Variables|Default|GetPreviewBuilding)))
        (Default|AddRemoveResources (CallFunction|GetPSRef) (.Cost (Utilities|Struct|BreakS_Crafteable (Variables|/Game/Blueprints/Buildings/BP_BaseBuilding.BP_BaseBuilding_C|GetCrafteableData (Variables|Default|GetPreviewBuilding)))) false)
        (CallFunction|CancelPreviewBuilding)))
    (:else)))

(event Custom|Build
  (params (IDBuilding :type Name))
  (Variables|Default|GetPreviewBuilding
    (:then)
    (:else
      (bind _returnvalue (Game|SpawnActorfromClass "/Game/Blueprints/Buildings/BP_BasePreviewBuilding.BP_BasePreviewBuilding_C" (Math|Transform|MakeTransform (CallFunction|GetCursorLocation "TraceTypeQuery4") "0, 0, 0" "1.000000,1.000000,1.000000") "Undefined" "MultiplyWithRoot" self IDBuilding "(R=0.000000,G=0.000000,B=0.000000,A=0.000000)" 0))
      (Variables|Default|SetPreviewBuilding _returnvalue))))

(event Input|EnhancedActionEvents|EnhancedInputActionIA_Build
  (params (ActionValue :type Boolean) (ElapsedSeconds :type Float%20%28double-precision%29) (TriggeredSeconds :type Float%20%28double-precision%29) (InputAction :type Input%20Action%20Object%20Reference :default "/Game/Inputs/IA_Build.IA_Build"))
  (:Started
    (CallFunction|Build "townhall")))

(event Input|EnhancedActionEvents|EnhancedInputActionIA_Select
  (params (ActionValue :type Vector%202D%20Structure) (ElapsedSeconds :type Float%20%28double-precision%29) (TriggeredSeconds :type Float%20%28double-precision%29) (InputAction :type Input%20Action%20Object%20Reference :default "/Game/Inputs/IA_Select.IA_Select"))
  (:Started
    (Variables|Default|GetPreviewBuilding
      (:then
        (CallFunction|ConfirmBuilding))
      (:else
        (Default|Select (CallFunction|GetPawnRef))))))

(event Input|EnhancedActionEvents|EnhancedInputActionIA_Order
  (params (ActionValue :type Vector%202D%20Structure) (ElapsedSeconds :type Float%20%28double-precision%29) (TriggeredSeconds :type Float%20%28double-precision%29) (InputAction :type Input%20Action%20Object%20Reference :default "/Game/Inputs/IA_Order.IA_Order"))
  (:Started
    (Variables|Default|GetPreviewBuilding
      (:then
        (CallFunction|CancelPreviewBuilding))
      (:else
        (Default|Order (CallFunction|GetPawnRef))))))

(fn ConstructionScript)

(fn GetPawnRef
  (Variables|References|GetPlayerPawn
    (:then
      _)
    (:else
      (bind _asbp_pawn_rts (Utilities|Casting|CastToBP_PawnRTS (Pawn|GetControlledPawn)))
      (Variables|References|SetPlayerPawn _asbp_pawn_rts)))
  (return (Variables|References|GetPlayerPawn)))

(fn GetCursorLocation
  (params (TraceChannel :type ETraceTypeQuery%20Enum :default "TraceTypeQuery1"))
  (return (.Location (Collision|BreakHitResult (.HitResult (Game|Player|GetHitResultUnderCursorbyChannel TraceChannel false))))))

(fn GetHudRef
  (Variables|References|GetHUD
    (:then
      _)
    (:else
      (bind _ashud_rts (Utilities|Casting|CastToHUD_RTS (HUD|GetHUD)))
      (Variables|References|SetHUD _ashud_rts)))
  (return (Variables|References|GetHUD)))

(fn GetGSRef
  (Variables|References|GetGameState
    (:then
      _)
    (:else
      (bind _asgs_rts (Utilities|Casting|CastToGS_RTS (Game|GetGameState)))
      (Variables|References|SetGameState _asgs_rts)))
  (return (Variables|References|GetGameState)))

(fn CancelPreviewBuilding
  (Actor|DestroyActor (Variables|Default|GetPreviewBuilding))
  (Variables|Default|SetPreviewBuilding 0))

(fn GetPSRef
  (Variables|Default|GetPS
    (:then
      _)
    (:else
      (bind _asps_rts (Utilities|Casting|CastToPS_RTS (Variables|GetPlayerState)))
      (Variables|Default|SetPS _asps_rts)))
  (return (Variables|Default|GetPS)))