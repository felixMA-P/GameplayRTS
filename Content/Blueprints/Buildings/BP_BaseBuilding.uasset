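; Base building actor for an RTS that snaps to a 100-unit grid and scales its collision to the building's footprint.
; Shortly after BeginPlay it loads its ID's rows from the building and craftable data tables, setting mesh, transform and a player-color dynamic material.
; It checks affordability through the cached local RTS PlayerState.
; On selection it returns UI data, actions and craftables.
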(event EventBeginPlay
  (Utilities|FlowControl|Delay 0.1)
  (CallFunction|SetBuildingValues))

(event Collision|EventActorBeginOverlap
  (params (OtherActor :type Actor%20Object%20Reference)))

(event EventTick
  (params (DeltaSeconds :type Float%20%28single-precision%29)))

(fn ConstructionScript
  (CallFunction|ScaleGridCollision)
  (CallFunction|ClamptoGrid (Transformation|GetActorLocation)))

(fn ClamptoGrid
  (params (InVec :type Vector))
  (bind (_x _y _z) (Math|Vector|BreakVector InVec))
  (Transformation|SetActorLocation (Math|Vector|MakeVector (Math|Conversions|ToFloat(Integer) (* (Math|Float|Round (/ _x 1e+02)) 100)) (Math|Conversions|ToFloat(Integer) (* (Math|Float|Round (/ _y 1e+02)) 100)) _z) false false))

(fn CorrectPivot
  (bind _buildingdata (Variables|Default|GetBuildingData))
  (bind (_x _y) (Math|Vector2D|BreakVector2D (.gridsize _buildingdata)))
  (Transformation|SetRelativeLocation (Variables|Default|GetPositionFixed) (Math|Vector|MakeVector (* _x 5e+01) (* _y 5e+01) 0.0) false false))

(fn ScaleGridCollision
  (bind _buildinggridcollision (Variables|Default|GetBuildingGridCollision))
  (bind _buildingdata (Variables|Default|GetBuildingData))
  (bind (_x _y) (Math|Vector2D|BreakVector2D (.gridsize _buildingdata)))
  (Transformation|SetRelativeScale3D _buildinggridcollision (Math|Vector|MakeVector (- _x 0.01) (- _y 0.01) (.z (Variables|/Script/Engine.SceneComponent|GetRelativeScale3D _buildinggridcollision)))))

(fn SetBuildingValues
  (Utilities|FlowControl|Sequence
    (:then_0
      (bind _returnvalue (Utilities|GetDataTableRow "/Game/DataTables/DT_Buildings.DT_Buildings" (Variables|Default|GetIDBuilding))
        (:then
          (Variables|Default|SetBuildingData _returnvalue)
          (CallFunction|ScaleGridCollision)
          (Transformation|SetRelativeTransform (Variables|Default|GetVisualMesh) (.RelativeTransform (Utilities|Struct|BreakS_Building _returnvalue)) false false)
          (Components|StaticMesh|SetStaticMesh (Variables|Default|GetVisualMesh) (.VisualMesh (Utilities|Struct|BreakS_Building _returnvalue)))
          (bind _returnvalue_2 (Rendering|Material|CreateDynamicMaterialInstance "/Game/Material/M_PlayerColor.M_PlayerColor" "PlayerColor" "None" :!class /Script/Engine.KismetMaterialLibrary))
          (bind _output_get (Variables|Default|SetBuildingPlayerMaterial _returnvalue_2))
          (Rendering|Material|SetMaterialbyName (Variables|Default|GetVisualMesh) (.MaterialStaticMeshName (Utilities|Struct|BreakS_Building _returnvalue)) _output_get)
          (Rendering|Material|SetVectorParameterValue (Variables|Default|GetBuildingPlayerMaterial) "BaseColorFactor" (Variables|Default|GetColor) :!class /Script/Engine.MaterialInstanceDynamic))))
    (:then_1
      (bind _returnvalue_3 (Utilities|GetDataTableRow "/Game/DataTables/DT_Crafteables.DT_Crafteables" (Variables|Default|GetIDBuilding))
        (:then
          (Variables|Default|SetCrafteableData _returnvalue_3))))))

(fn CanIPayIt
  (return (Default|CanIPayIt (CallFunction|GetLocalPSRef) (.Cost (Utilities|Struct|BreakS_Crafteable (Variables|Default|GetCrafteableData))))))

(fn GetLocalPSRef
  (Variables|Default|GetPS
    (:then
      _)
    (:else
      (bind _asps_rts (Utilities|Casting|CastToPS_RTS (Game|GetPlayerState 0)))
      (Variables|Default|SetPS _asps_rts)))
  (return (Variables|Default|GetPS)))

(fn Select
  (bind _returnvalue (Utilities|GetDataTableRow "/Game/DataTables/DT_Buildings.DT_Buildings" (Variables|Default|GetIDBuilding))
    (:then
      (return (Utilities|Struct|MakeS_SelectedUIData (Variables|Default|GetRow%20Name) "NewEnumerator0" "NewEnumerator0" (Variables|Default|GetSoftMiniature) (Variables|Default|GetAtt%20Map)) (.Actions (Utilities|Struct|BreakS_Building _returnvalue)) (.Crafteables (Utilities|Struct|BreakS_Building _returnvalue))))))