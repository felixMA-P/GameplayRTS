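; Base placement preview for RTS buildings that follows the cursor, clamped to a grid, and shows whether the building can be placed.
; Each tick snaps it to the RTS controller's cursor hit and sets the grid material's Status parameter from placement and affordability checks.
; Placement requires the grid collision to overlap nothing but BP_BaseZone actors, whose gameplay tags must cover any zones required by BuildingData.
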(event EventBeginPlay
  (|CallParentFunction)
  (bind _returnvalue (Rendering|Material|CreateDynamicMaterialInstance "/Game/Material/BuildingPreviewMaterial.BuildingPreviewMaterial" "None" "None" :!class /Script/Engine.KismetMaterialLibrary))
  (bind _output_get (Variables|Default|SetGridMaterialInstance _returnvalue))
  (Rendering|Material|SetMaterial (Variables|Default|GetBuildingGridCollision) 0 _output_get))

(event Collision|EventActorBeginOverlap
  (params (OtherActor :type Actor%20Object%20Reference))
  (|CallParentFunction OtherActor) ; This node is disabled and will not be called.\nDrag off pins to build functionality.
)

(event EventTick
  (params (DeltaSeconds :type Float%20%28single-precision%29))
  (CallFunction|ClamptoGrid (Default|GetCursorLocation (CallFunction|GetPCRts) "TraceTypeQuery4"))
  (CallFunction|ChangeMaterialColorBuildingGrid))

(fn ConstructionScript
  (|CallParentFunction))

(fn GetPCRts
  (Variables|Default|GetPCRTS
    (:then
      _)
    (:else
      (bind _aspc_rts (Utilities|Casting|CastToPC_RTS (Game|GetPlayerController 0)))
      (Variables|Default|SetPCRTS _aspc_rts)))
  (return (Variables|Default|GetPCRTS)))

(fn CaniBuildHere
  (bind _buildinggridcollision (Variables|Default|GetBuildingGridCollision))
  (bind _overlappingactors (Collision|GetOverlappingActors _buildinggridcollision 0 :!class /Script/Engine.PrimitiveComponent))
  (return (and (or (Utilities|Array|IsEmpty _overlappingactors) (== (Utilities|Array|Length _overlappingactors) (Utilities|Array|Length (Collision|GetOverlappingActors (Variables|Default|GetBuildingGridCollision) "/Game/Blueprints/BuildingZones/BP_BaseZone.BP_BaseZone_C" :!class /Script/Engine.PrimitiveComponent)))) (CallFunction|CheckConstructionTags))))

(fn ChangeMaterialColorBuildingGrid
  (Rendering|Material|SetScalarParameterValue (Variables|Default|GetGridMaterialInstance) "Status" (select (and (CallFunction|CaniBuildHere) (CallFunction|CanIPayIt)) 1.0 0.0) :!class /Script/Engine.MaterialInstanceDynamic))

(fn CheckConstructionTags
  (if (> (GameplayTags|GetNumGameplayTagsinContainer (.neededconstructzone (Variables|Default|GetBuildingData))) 0)
    (for (_array_element _array_index) (Collision|GetOverlappingActors (Variables|Default|GetBuildingGridCollision) "/Game/Blueprints/BuildingZones/BP_BaseZone.BP_BaseZone_C" :!class /Script/Engine.PrimitiveComponent)
      (bind _asbp_base_zone (Utilities|Casting|CastToBP_BaseZone _array_element))
      (GameplayTags|AddGameplayTag (LocalVariables|GetCheckerGameplay) (Variables|/Game/Blueprints/BuildingZones/BP_BaseZone.BP_BaseZone_C|GetGameplayTag _asbp_base_zone) :!class /Script/GameplayTags.BlueprintGameplayTagLibrary)
      (Development|PrintString (Utilities|String|ToString(Name) (GameplayTags|GetTagName (Variables|/Game/Blueprints/BuildingZones/BP_BaseZone.BP_BaseZone_C|GetGameplayTag _asbp_base_zone))) true false "(R=0.000000,G=0.660000,B=1.000000,A=1.000000)" 0.1 (Utilities|String|StringToName (Utilities|String|ToString(Integer) _array_index))))
    (return (and (GameplayTags|HasAllTags (LocalVariables|GetCheckerGameplay) (.neededconstructzone (Variables|Default|GetBuildingData))) (> (GameplayTags|GetNumGameplayTagsinContainer (LocalVariables|GetCheckerGameplay)) 0)))
    (else
      (return true))))