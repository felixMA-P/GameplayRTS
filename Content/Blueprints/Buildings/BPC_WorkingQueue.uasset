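; Building component that runs a paid, timed production queue of craftables, requesting units from the owning player's PS_RTS.
; Adding an entry calls PayForCrafteableServer and queues it only if paid, starting processing when idle.
; The head entry's DT_Crafteables craft time sets a timer, which requests the unit at zero location, then advances the queue.
; CancelLastAddedElement actually removes the first entry, without refunding or clearing the timer.
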(event Custom|CancelLastAddedElement
  (if (not (Utilities|Array|IsEmpty (Variables|Default|GetQueue)))
    (Utilities|Array|RemoveIndex (Variables|Default|GetQueue))))

(event Custom|TryAddElementToQueue
  (params (CrafteableName :type Name%20%28by%20ref%29))
  (bind _bpaid (Default|PayforCrafteableServer (CallFunction|GetPSRef) CrafteableName))
  (if _bpaid
    (Utilities|Array|Add (Variables|Default|GetQueue) CrafteableName)
    (if (not (Variables|Default|GetbIsRuning))
      (CallFunction|TrytoSpawn)
      (Variables|Default|SetbIsRuning true))))

(event Custom|RemoveFirstElementFormQueue
  (Utilities|Array|RemoveIndex (Variables|Default|GetQueue)))

(event Custom|Spawn%20class
  (if (not (Utilities|Array|IsEmpty (Variables|Default|GetQueue)))
    (Default|AskforCreateUnit (CallFunction|GetPSRef) (Utilities|Array|Get(acopy) (Variables|Default|GetQueue)) "0, 0, 0")
    (CallFunction|RemoveFirstElementFormQueue)
    (Utilities|Time|ClearandInvalidateTimerbyHandle (Variables|Default|GetTimer))
    (CallFunction|TrytoSpawn)))

(event Custom|TryToSpawn
  (if (Utilities|Array|IsEmpty (Variables|Default|GetQueue))
    (Variables|Default|SetbIsRuning false)
    (else
      (bind _returnvalue (Utilities|GetDataTableRow "/Game/DataTables/DT_Crafteables.DT_Crafteables" (Utilities|Array|Get(acopy) (Variables|Default|GetQueue)))
        (:then
          (bind _output_get (Variables|Default|SetCurrentCrafteable _returnvalue))
          (bind _returnvalue_2 (Utilities|Time|SetTimerbyEvent (delegate Custom|Spawn%20class) (Utilities|Struct|BreakS_Crafteable _output_get)))
          (Variables|Default|SetTimer _returnvalue_2))))))

(event EventBeginPlay)

(event EventTick
  (params (DeltaSeconds :type Float%20%28single-precision%29)))

(fn GetPSRef
  (Variables|Default|GetPS%20RTS
    (:then
      _)
    (:else
      (bind _aspc_rts (Utilities|Casting|CastToPC_RTS (Components|GetOwner (Components|GetOwner))))
      (bind _asps_rts (Utilities|Casting|CastToPS_RTS (Variables|/Script/Engine.Controller|GetPlayerState _aspc_rts)))
      (Variables|Default|SetPS%20RTS _asps_rts)))
  (return (Variables|Default|GetPS%20RTS)))