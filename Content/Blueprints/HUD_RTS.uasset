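; HUD_RTS is the RTS HUD that creates the main UI widget and relays selection, action and resource updates to it.
; Selection events fill the unit, action and craftable displays, while RefreshResources updates the resource panel.
; It adds and removes a craftable hover-info widget anchored to the right of the main canvas.
; Craft requests go to the player state's queue through GetPSRef, which lazily caches the PS_RTS cast.
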(event Custom|SomthingSelected
  (params (UIStruct :type S%20Selected%20UI%20Data%20Structure) (InActions :type Array%20of%20E_Actions%20Enums :default "NewEnumerator0") (Crafteables :type Array%20of%20Names))
  (Default|OnUnitSelected (Variables|Default|GetMainUI) UIStruct)
  (Default|SetActions (Variables|Default|GetMainUI) InActions Crafteables))

(event Custom|CreateCrafteableInfo
  (params (S%20Crafteable :type S%20Crafteable%20Structure))
  (bind _returnvalue (Game|ConstructObjectfromClass "/Game/UI/Main/Crafteables/UW_CrafteableHoverInfo.UW_CrafteableHoverInfo_C" S%20Crafteable))
  (Variables|Default|SetCrafteableHover _returnvalue)
  (bind _returnvalue_2 (Class|CanvasPanel|AddChildtoCanvas (Variables|/Game/UI/Main/UW_Main.UW_Main_C|GetMainCanvas (Variables|Default|GetMainUI)) _returnvalue))
  (Class|CanvasPanelSlot|SetAnchors _returnvalue_2 (Utilities|Struct|MakeAnchors "(X=1.000000,Y=0.145000)" "(X=1.000000,Y=0.145000)"))
  (Class|CanvasPanelSlot|SetPosition _returnvalue_2 "(X=-50.000000,Y=0.000000)")
  (Class|CanvasPanelSlot|SetAlignment _returnvalue_2 "(X=1.000000,Y=0.000000)")
  (Class|CanvasPanelSlot|SetSize _returnvalue_2 "(X=500.000000,Y=500.000000)"))

(event Custom|DeleteCrafteableHover
  (Widget|RemovefromParent (Variables|Default|GetCrafteableHover))
  (Variables|Default|SetCrafteableHover 0))

(event Custom|CreateSomething
  (params (CrafteableID :type Name))
  (Default|TryAddNewElementtoQueue (CallFunction|GetPSRef) CrafteableID))

(event EventBeginPlay
  (bind _returnvalue (UserInterface|CreateWidget "/Game/UI/Main/UW_Main.UW_Main_C"))
  (bind _output_get (Variables|Default|SetMainUI _returnvalue))
  (UserInterface|Viewport|AddtoViewport _output_get 0))

(event Collision|EventActorBeginOverlap
  (params (OtherActor :type Actor%20Object%20Reference)))

(event EventTick
  (params (DeltaSeconds :type Float%20%28single-precision%29)))

(fn ConstructionScript)

(fn RefreshResources
  (params (Resources :type Array%20of%20E_ResourcesTypes%20Enums :default "NewEnumerator0") (Quantities :type Array%20of%20Integers))
  (bind _mainui (Variables|Default|GetMainUI)
    (:then
      (Default|RefreshValues (Variables|/Game/UI/Main/UW_Main.UW_Main_C|GetUW_Resources _mainui) Resources Quantities))
    (:else
      (Development|PrintString "No vale majo"))))

(fn SetActions
  (params (InActions :type Array%20of%20E_Actions%20Enums :default "NewEnumerator0"))
  (Default|SetActions (Variables|Default|GetMainUI) InActions))

(fn GetPSRef
  (Variables|Default|GetPS
    (:then
      _)
    (:else
      (bind _asps_rts (Utilities|Casting|CastToPS_RTS (Game|GetPlayerState 0)))
      (Variables|Default|SetPS _asps_rts)))
  (return (Variables|Default|GetPS)))