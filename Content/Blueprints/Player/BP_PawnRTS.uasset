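; RTS player pawn that handles camera movement, cursor selection, order feedback, pings and queuing craftables on the selected actor's BPC_WorkingQueue.
; Cursor traces drive selection, which passes the actor's UI data to PC_RTS and multicasts a bounds-scaled, player-colored decal.
; Right-click orders only spawn a feedback cursor, and pings spawn through server events.
; Zoom changes spring arm length and steps its pitch.
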(event EventBeginPlay)

(event Collision|EventActorBeginOverlap
  (params (OtherActor :type Actor%20Object%20Reference)))

(event EventTick
  (params (DeltaSeconds :type Float%20%28single-precision%29)))

(event Custom|SpawnFeedBackOnServer
  (params (Spawn%20Transform%20Location :type Vector))
  (bind _pc (CallFunction|GetPCRef))
  (Game|SpawnActorfromClass "/Game/Blueprints/Player/BP_FeedBackCursor.BP_FeedBackCursor_C" (Math|Transform|MakeTransform Spawn%20Transform%20Location "0, 0, 0" "1.000000,1.000000,1.000000") "AlwaysSpawn" "MultiplyWithRoot" 0 (Variables|/Game/Blueprints/PC_RTS.PC_RTS_C|GetPlayerName _pc) (Variables|/Game/Blueprints/PC_RTS.PC_RTS_C|GetPlayerColor _pc) 0))

(event Custom|Select
  (bind _pc (CallFunction|GetPCRef))
  (bind (_worldlocation _worlddirection) (Game|Player|ConvertMouseLocationToWorldSpace _pc))
  ;[1 1 1] Click izq
  (bind (_outhit _returnvalue) (Collision|LineTraceByChannel _worldlocation (+ _worldlocation (* _worlddirection 1e+04)) "TraceTypeQuery3" false 0 "None"))
  (if _returnvalue
    (CallFunction|DeselectElement)
    (bind (_uidata _actions _crafteables) (Class|BPISelectable|Select(Message) (.HitActor (Collision|BreakHitResult _outhit))))
    (Default|UIonSelectableSelected (CallFunction|GetPCRef) _uidata _actions _crafteables)
    (CallFunction|SelectElementonServer (.HitActor (Collision|BreakHitResult _outhit)))
    (Variables|Default|SetSelectedActor (.HitActor (Collision|BreakHitResult _outhit)))
    (else
      (CallFunction|DeselectElement))))

(event Custom|Order
  (bind _pc (CallFunction|GetPCRef))
  (bind (_worldlocation _worlddirection) (Game|Player|ConvertMouseLocationToWorldSpace _pc))
  ;[1 1 1] Click Der
  (bind (_outhit _returnvalue) (Collision|LineTraceByChannel _worldlocation (+ _worldlocation (* _worlddirection 1e+04)) "TraceTypeQuery3" false 0 "None"))
  (if _returnvalue
    (CallFunction|SpawnFeedBackonServer (.Location (Collision|BreakHitResult _outhit)))))

(event Custom|SelectElementOnServer
  (params (Actor :type Actor%20Object%20Reference))
  (CallFunction|AddDecalEffectMulticast Actor (Variables|/Game/Blueprints/PC_RTS.PC_RTS_C|GetPlayerColor (CallFunction|GetPCRef))))

(event Custom|AddDecalEffectMulticast
  (params (Actor :type Actor%20Object%20Reference) (Value :type Linear%20Color%20Structure))
  (bind _boxextent (Collision|GetActorBounds Actor true false))
  (bind _returnvalue (> (.x _boxextent) (.y _boxextent)))
  (bind _returnvalue_2 (Math|Float|SelectFloat (.x _boxextent) (.y _boxextent) _returnvalue))
  (bind _returnvalue_3 (/ _returnvalue_2 8e+01))
  (bind _returnvalue_4 (Math|Float|Clamp(Float) _returnvalue_3 1.0 1e+01))
  (bind _returnvalue_5 (AddComponent|AddDecalComponent Actor false (Math|Transform|MakeTransform "0, 0, 0" "90.000000,0.000000,0.000000" (Math|Vector|MakeVector 1.0 _returnvalue_4 _returnvalue_4))))
  (bind _returnvalue_6 (Rendering|Material|CreateDynamicMaterialInstance "/Game/Material/Decal/M_Selected.M_Selected" "None" "None" :!class /Script/Engine.KismetMaterialLibrary))
  (Rendering|Material|SetVectorParameterValue _returnvalue_6 "Color" Value :!class /Script/Engine.MaterialInstanceDynamic)
  (Rendering|Components|Decal|SetDecalMaterial _returnvalue_5 _returnvalue_6))

(event Custom|RemoveSelectedDecalOnServer
  (params (Target :type Actor%20Object%20Reference))
  (CallFunction|RemoveDecalMulticast Target))

(event Custom|RemoveDecalMulticast
  (params (Target :type Actor%20Object%20Reference))
  (bind _returnvalue (Actor|GetComponentbyClass Target "/Script/Engine.DecalComponent"))
  (Transformation|DetachFromComponent _returnvalue "KeepRelative" "KeepRelative" "KeepRelative" true)
  (Components|DestroyComponent _returnvalue))

(event Custom|AddElementToQueue
  (params (CrafteableName :type Name%20%28by%20ref%29))
  (if (Utilities|IsValid (Variables|Default|GetSelectedActor))
    (Default|AddElementtoQueue (Actor|GetComponentbyClass (Variables|Default|GetSelectedActor) "/Game/Blueprints/Buildings/BPC_WorkingQueue.BPC_WorkingQueue_C") CrafteableName)))

(event Custom|SpawnPingOnServer
  (params (Spawn%20Transform%20Location :type Vector))
  (bind _returnvalue (Game|SpawnActorfromClass "/Game/Blueprints/Player/Pings/BP_Ping.BP_Ping_C" (Math|Transform|MakeTransform Spawn%20Transform%20Location "0.000000,180.000000,0.000000" "1.000000,1.000000,1.000000") "Undefined" "MultiplyWithRoot" (CallFunction|GetPCRef) 0))
  (Variables|Default|SetPing _returnvalue))

(event Custom|DestroyPingOnServer
  (if (not (Variables|/Game/Blueprints/Player/Pings/BP_Ping.BP_Ping_C|GetbIsNiagaraActive (Variables|Default|GetPing)))
    (bind _ping (Variables|Default|GetPing)
      (:then
        (Actor|DestroyActor _ping))
      (:else))))

(event Input|EnhancedActionEvents|EnhancedInputActionIA_Ping
  (params (ActionValue :type Boolean) (ElapsedSeconds :type Float%20%28double-precision%29) (TriggeredSeconds :type Float%20%28double-precision%29) (InputAction :type Input%20Action%20Object%20Reference :default "/Game/Inputs/IA_Ping.IA_Ping"))
  (:Started
    (CallFunction|SpawnPingonServer (Default|GetCursorLocation (CallFunction|GetPCRef) "TraceTypeQuery4")))
  (:Canceled
    (CallFunction|DestroyPingonServer :!label _label))
  (:Completed
    (goto _label)))

(event Input|EnhancedActionEvents|EnhancedInputActionIA_Movement
  (params (ActionValue :type Vector%202D%20Structure) (ElapsedSeconds :type Float%20%28double-precision%29) (TriggeredSeconds :type Float%20%28double-precision%29) (InputAction :type Input%20Action%20Object%20Reference :default "/Game/Inputs/IA_Movement.IA_Movement"))
  (Class|PawnMovementComponent|AddInputVector (Variables|Default|GetFloatingPawnMovement) (Math|Conversions|ToVector(Vector2D) ActionValue) false))

(event Input|EnhancedActionEvents|EnhancedInputActionIA_Zoom
  (params (ActionValue :type Float%20%28double-precision%29) (ElapsedSeconds :type Float%20%28double-precision%29) (TriggeredSeconds :type Float%20%28double-precision%29) (InputAction :type Input%20Action%20Object%20Reference :default "/Game/Inputs/IA_Zoom.IA_Zoom"))
  (bind _springarm (Variables|Default|GetSpringArm))
  (bind _springarm_2 (Variables|Default|GetSpringArm))
  (bind _relativerotation (Variables|/Script/Engine.SceneComponent|GetRelativeRotation _springarm))
  (bind _relativerotation_2 (Variables|/Script/Engine.SceneComponent|GetRelativeRotation _springarm_2))
  (if (and (< (+ (* ActionValue 5e+01) (Variables|/Script/Engine.SpringArmComponent|GetTargetArmLength (Variables|Default|GetSpringArm))) 2e+03) (> (+ (* ActionValue 5e+01) (Variables|/Script/Engine.SpringArmComponent|GetTargetArmLength (Variables|Default|GetSpringArm))) 1e+02))
    (Variables|/Script/Engine.SpringArmComponent|SetTargetArmLength (Variables|Default|GetSpringArm) (+ (* ActionValue 5e+01) (Variables|/Script/Engine.SpringArmComponent|GetTargetArmLength (Variables|Default|GetSpringArm))))
    (if (< ActionValue 0.0)
      (if (and (< (.pitch (Variables|/Script/Engine.SceneComponent|GetRelativeRotation (Variables|Default|GetSpringArm))) -2e+01) (< (Variables|/Script/Engine.SpringArmComponent|GetTargetArmLength (Variables|Default|GetSpringArm)) 5e+02))
        (Transformation|SetRelativeRotation (Variables|Default|GetSpringArm) (Math|Rotator|MakeRotator (.roll _relativerotation_2) (+ (.pitch _relativerotation_2) 1e+01) (.yaw _relativerotation_2)) false false))
      (elif (and (!= (.pitch (Variables|/Script/Engine.SceneComponent|GetRelativeRotation (Variables|Default|GetSpringArm))) -9e+01) (> (Variables|/Script/Engine.SpringArmComponent|GetTargetArmLength (Variables|Default|GetSpringArm)) 1e+02))
        (Transformation|SetRelativeRotation (Variables|Default|GetSpringArm) (Math|Rotator|MakeRotator (.roll _relativerotation) (+ (.pitch _relativerotation) -1e+01) (.yaw _relativerotation)) false false)))))

(fn ConstructionScript)

(fn GetPCRef
  (Variables|Default|GetPC_RTS
    (:then
      _)
    (:else
      (bind _aspc_rts (Utilities|Casting|CastToPC_RTS (Components|GetOwner)))
      (Variables|Default|SetPC_RTS _aspc_rts)))
  (return (Variables|Default|GetPC_RTS)))

(fn DeselectElement
  (bind _selectedactor (Variables|Default|GetSelectedActor)
    (:then
      (Class|BPISelectable|DeSelect(Message) _selectedactor)
      (CallFunction|RemoveSelectedDecalonServer _selectedactor))
    (:else)))

(fn GetPSRef
  (Variables|Default|GetPS_RTS
    (:then
      _)
    (:else
      (bind _asps_rts (Utilities|Casting|CastToPS_RTS (Variables|/Script/Engine.Controller|GetPlayerState (CallFunction|GetPCRef))))
      (Variables|Default|SetPS_RTS _asps_rts)))
  (return (Variables|Default|GetPS_RTS)))