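; BP_FeedBackCursor is a short-lived cursor feedback actor that displays a player name alongside a Niagara effect tinted in a given color.
; On BeginPlay it calls ServerSetValues, which forwards to MulticastSetValues to apply the Name text and Color parameter, apparently for replication to all clients.
; It sets a one-second lifespan, so each marker removes itself automatically.
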(event Custom|MulticastSetValues
  (Rendering|Components|TextRender|SetText (Variables|Default|GetPlayerName) (Variables|Default|GetName))
  (Effects|Components|ParticleSystem|SetColorParameter (Variables|Default|GetNiagara) "Color" (Variables|Default|GetColor)))

(event Custom|ServerSetValues
  (CallFunction|MulticastSetValues))

(event EventBeginPlay
  (CallFunction|ServerSetValues)
  (Actor|SetLifeSpan 1.0))

(event Collision|EventActorBeginOverlap
  (params (OtherActor :type Actor%20Object%20Reference)))

(event EventTick
  (params (DeltaSeconds :type Float%20%28single-precision%29)))

(fn ConstructionScript)