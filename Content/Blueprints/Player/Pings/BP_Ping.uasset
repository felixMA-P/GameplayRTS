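; BP_Ping is a player ping actor that lets its owner pick a ping type, then plays the matching effect.
; On BeginPlay, it shows its UW_Ping widget only if the owner is the first player controller, initializing it with the MapPings table.
; A click looks up that type's Niagara asset, passes it through ActivateNiagaraOnServer to ActivateNiagara, and hides the widget.
; The actor destroys itself shortly after the effect starts.
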(event Custom|ActivateNiagara
  (params (InAsset :type Niagara%20System%20Object%20Reference))
  (Class|NiagaraComponent|SetAsset (Variables|Default|GetNiagara) InAsset true)
  (Variables|Default|SetbIsNiagaraActive true)
  (Components|Activation|Activate (Variables|Default|GetNiagara) false)
  (Utilities|FlowControl|Delay 1.0)
  (Actor|DestroyActor))

(event Custom|SelectPingType
  (params (Ping :type E_PingTypes%20Enum :default "NewEnumerator4"))
  (bind _output_get (Variables|Default|SetPingType Ping))
  (if (.ReturnValue (Utilities|Map|Find (Variables|Default|GetMapPings) _output_get))
    (CallFunction|ActivateNiagaraonServer (.Value (Utilities|Map|Find (Variables|Default|GetMapPings) _output_get)))
    (Rendering|SetVisibility (Variables|Default|GetWidget) false false)
    (else
      (Development|PrintString "Error ping not found"))))

(event Custom|ActivateNiagaraOnServer
  (params (InAsset :type Niagara%20System%20Object%20Reference))
  (CallFunction|ActivateNiagara InAsset))

(event EventBeginPlay
  (if (== (Components|GetOwner) (Game|GetPlayerController 0))
    (Rendering|SetVisibility (Variables|Default|GetWidget) true false)
    (bind _asuw_ping (Utilities|Casting|CastToUW_Ping (UserInterface|GetWidget (Variables|Default|GetWidget))))
    (Default|Initialize _asuw_ping (Variables|Default|GetMapPings))
    (EventDispatchers|BindEventtoOnPingClicked _asuw_ping (delegate Custom|SelectPingType))))

(event Collision|EventActorBeginOverlap
  (params (OtherActor :type Actor%20Object%20Reference)))

(event EventTick
  (params (DeltaSeconds :type Float%20%28single-precision%29)))

(fn ConstructionScript)