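; World-space cursor actor that displays a player's name in their color, hiding its visuals from the owning local player.
; On BeginPlay a server event multicasts the name and color to the text component.
; SetCustomNewLocation stores a target, delta time and speed, then restarts a looping timer at that interval, apparently driving InterpolateToLocation to ease the actor there with VInterpTo instead of using Tick.
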(event Custom|MulticastSetValues
  (Rendering|Components|TextRender|SetTextRenderColor (Variables|Default|GetWName) (Math|Conversions|ToColor(LinearColor) (Variables|Default|GetColor)))
  (Rendering|Components|TextRender|SetText (Variables|Default|GetWName) (Variables|Default|GetName)))

(event Custom|ServerSetValues
  (CallFunction|MulticastSetValues))

(event Custom|SetCustomNewLocation
  (params (NewLocation :type Vector) (Delta%20Time :type Float%20%28single-precision%29) (Interp%20Speed :type Float%20%28single-precision%29))
  (Variables|Default|SetNew%20Location NewLocation)
  (Variables|Default|SetDelta%20Time Delta%20Time)
  (Variables|Default|SetInterp%20Speed Interp%20Speed)
  (if (and (Utilities|Time|IsValidTimerHandle (Variables|Default|GetTimer)) (Utilities|Time|IsTimerActivebyHandle (Variables|Default|GetTimer)))
    (Utilities|Time|ClearandInvalidateTimerbyHandle (Variables|Default|GetTimer))
    (Variables|Default|SetTimer (Variables|Default|GetTimer)))
  (bind _returnvalue (Utilities|Time|SetTimerbyEvent (EventDispatchers|CreateEvent :!event Custom|InterpolateToLocation) (Variables|Default|GetDelta%20Time) true))
  (Variables|Default|SetTimer _returnvalue))

(event Custom|InterpolateToLocation
  (Transformation|SetActorLocation (Math|Interpolation|VInterpTo (Transformation|GetActorLocation) (Variables|Default|GetNew%20Location) (Variables|Default|GetDelta%20Time) (Variables|Default|GetInterp%20Speed)) false false))

(event EventBeginPlay
  (CallFunction|ServerSetValues)
  (if (== (Game|GetPlayerController 0) (Components|GetOwner))
    (Rendering|SetVisibility (Variables|Default|GetDefaultSceneRoot) false true)))

(event Collision|EventActorBeginOverlap
  (params (OtherActor :type Actor%20Object%20Reference)))

(event EventTick
  (params (DeltaSeconds :type Float%20%28single-precision%29)))

(fn ConstructionScript)