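; RTS GameState that starts the match for players and spawns their buildings and units.
; StartGame waits briefly, then walks PlayerArray and tells each PC_RTS to spawn its world cursor.
; SpawnBuildForPlayer creates a BP_BaseDefinitiveBuilding owned by the given controller, with its building ID and player color.
; SpawnUnitForPlayer creates a BP_BaseUnit from a row name and location, without setting an owner or using its SCrafteable input.
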(event Custom|StartGame
  (Utilities|FlowControl|Delay 1.0)
  (for _array_element (Variables|Default|GetPlayerArray)
    (bind _aspc_rts (Utilities|Casting|CastToPC_RTS (Game|GetPlayerController _array_element)))
    (Default|SpawnWorldCursor _aspc_rts)))

(event Custom|SpawnBuildForPlayer
  (params (PC :type PC%20RTS%20Object%20Reference) (IDBuilding :type Name) (Spawn%20Transform%20Location :type Vector))
  (Game|SpawnActorfromClass "/Game/Blueprints/Buildings/BP_BaseDefinitiveBuilding.BP_BaseDefinitiveBuilding_C" (Math|Transform|MakeTransform Spawn%20Transform%20Location "0, 0, 0" "1.000000,1.000000,1.000000") "Undefined" "MultiplyWithRoot" PC IDBuilding (Variables|/Game/Blueprints/PC_RTS.PC_RTS_C|GetPlayerColor PC) 0))

(event Custom|SpawnUnitForPlayer
  (params (S_Crafteable :type S%20Crafteable%20Structure%20%28by%20ref%29) (Location :type Vector) (RowName :type Name))
  (Game|SpawnActorfromClass "/Game/Blueprints/Units/BP_BaseUnit.BP_BaseUnit_C" (Math|Transform|MakeTransform Location "0, 0, 0" "1.000000,1.000000,1.000000") "Undefined" "MultiplyWithRoot" 0 RowName 0))

(event EventTick
  (params (DeltaSeconds :type Float%20%28single-precision%29)))

(event EventBeginPlay)

(fn ConstructionScript)