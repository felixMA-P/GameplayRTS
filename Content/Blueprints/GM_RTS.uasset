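; GM_RTS is the RTS game mode that sets up joining players and starts the match once enough have arrived.
; Each new player's PC_RTS gets a color from the Colors array and a numbered name based on the current player count.
; When the count reaches Players, it marks the game started and calls StartGame on GS_RTS, fetched through a lazily cached getter.
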(event EventHandleStartingNewPlayer
  (params (NewPlayer :type Player%20Controller%20Object%20Reference))
  (|CallParentFunction NewPlayer)
  (bind _returnvalue (Class|GameModeBase|GetNumPlayers))
  (bind _aspc_rts (Utilities|Casting|CastToPC_RTS NewPlayer))
  (Variables|/Game/Blueprints/PC_RTS.PC_RTS_C|SetPlayerColor _aspc_rts (Utilities|Array|Get(acopy) (Variables|Default|GetColors) (- _returnvalue 1)))
  (Variables|/Game/Blueprints/PC_RTS.PC_RTS_C|SetPlayerName _aspc_rts (Utilities|Text|FormatText "Player {PlayerNum}" (Utilities|String|ToString(Integer) _returnvalue)))
  (if (>= _returnvalue (Variables|Default|GetPlayers))
    (Variables|Default|SetbGameStarted true)
    (Default|StartGame (CallFunction|GetGameStateRef))))

(event EventTick
  (params (DeltaSeconds :type Float%20%28single-precision%29)))

(event EventBeginPlay)

(fn ConstructionScript)

(fn GetGameStateRef
  (Variables|Default|GetGameStateRef
    (:then
      _)
    (:else
      (bind _asgs_rts (Utilities|Casting|CastToGS_RTS (Game|GetGameState)))
      (Variables|Default|SetGameStateRef _asgs_rts)))
  (return (Variables|Default|GetGameStateRef)))